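; Blueprint actor that applies a shared terrain material to actors tagged as VHM terrain tiles.
; ApplyToAllTiles sets TerrainMaterial on slot 0 of each tile's tagged Virtual Heightfield Mesh and Procedural Mesh components, printing a warning if the material is invalid.
; The initial call and looping re-apply timer are disconnected and BeginPlay is empty, so nothing in this Blueprint invokes the function.
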(event EventBeginPlay)

(event EventEndPlay
  (params (EndPlayReason :type EEndPlayReason%20Enum :default "Destroyed")))

(fn ConstructionScript)

(fn ApplytoAllTiles
  (bind _terrainmaterial (Variables|Default|GetTerrainMaterial))
  (Utilities|IsValid (Variables|Default|GetTerrainMaterial)
    (:Is%20Valid
      (bind _outactors (Actor|GetAllActorsOfClasswithTag "/Script/Engine.Actor" "VHMTerrainTile"))
      (for _array_element _outactors
        (Utilities|FlowControl|Sequence
          (:then_0
            (for _array_element_2 (Actor|GetComponentsbyTag _array_element "/Script/VirtualHeightfieldMesh.VirtualHeightfieldMeshComponent" "VHMRoot")
              (Rendering|Material|SetMaterial _array_element_2 0 _terrainmaterial)))
          (:then_1
            (for _array_element_3 (Actor|GetComponentsbyTag _array_element "/Script/ProceduralMeshComponent.ProceduralMeshComponent" "VHMProcMesh")
              (Rendering|Material|SetMaterial _array_element_3 0 _terrainmaterial))))))
    (:Is%20Not%20Valid
      (Development|PrintString "Material not set!" true true "(R=0.000000,G=0.660000,B=1.000000,A=1.000000)" 1e+01))))